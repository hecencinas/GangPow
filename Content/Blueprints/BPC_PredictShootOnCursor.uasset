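; Actor component that previews a projectile arc from its owner to the point under the mouse cursor.
; While enabled, each tick it solves a custom-arc launch velocity to the cursor hit, predicts the path and writes it into a runtime-added spline.
; An attached Niagara path effect is spawned on that spline.
; It also turns the owner to face the cursor, and disabling clears the spline.
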(event EventBeginPlay
  (bind _returnvalue (Game|AddComponentbyClass (Components|GetOwner) "/Script/Engine.SplineComponent" false))
  (bind _output_get (Variables|Default|SetSpline _returnvalue))
  (Spline|SetSplinePoints _output_get (Utilities|Array|MakeArray) "Local" true)
  (Niagara|SpawnSystemAttached "/Game/Blueprints/NS_ProjectilePath.NS_ProjectilePath" _output_get "None" "0, 0, 0" "0, 0, 0" "SnapToTarget" false true "AutoRelease"))

(event EventTick
  (params (DeltaSeconds :type Float%20%28single-precision%29))
  (if (Variables|Default|GetEnabled)
    (CallFunction|UpdateShootPreview)))

(fn UpdateShootPreview
  (bind _returnvalue (Components|GetOwner))
  (bind _returnvalue_2 (Components|GetOwner))
  (bind _returnvalue_3 (Game|GetPlayerController 0))
  (bind _array (Utilities|Array|MakeArray "ObjectTypeQuery7" "ObjectTypeQuery1"))
  (bind _returnvalue_4 (Transformation|GetActorLocation _returnvalue_2))
  (bind _returnvalue_5 (Transformation|GetActorLocation _returnvalue))
  (bind _hitresult (Class|PlayerController|GetHitResultUnderCursorforObjects _returnvalue_3 _array true))
  (bind (_x _y) (Math|Vector|BreakVector (.impactpoint _hitresult)))
  (bind _outlaunchvelocity (Game|SuggestProjectileVelocityCustomArc _returnvalue_5 (.impactpoint _hitresult) 0.0 0.5))
  (bind _outpathpositions (Class|GameplayStatics|BlueprintPredictProjectilePathbyTraceChannel _returnvalue_5 _outlaunchvelocity true 1.0 "ECC_Visibility" false (Utilities|Array|MakeArray _returnvalue) "None"))
  (Spline|SetSplinePoints (Variables|Default|GetSpline) _outpathpositions "World" true)
  (Transformation|SetActorRotation _returnvalue_2 (Math|Rotator|FindLookatRotation (Math|Vector|MakeVector (.x _returnvalue_4) (.y _returnvalue_4) 0.0) (Math|Vector|MakeVector _x _y 0.0))))

(fn Enable
  (Variables|Default|SetEnabled true))

(fn Disable
  (Variables|Default|SetEnabled false)
  (Spline|SetSplinePoints (Variables|Default|GetSpline) (Utilities|Array|MakeArray) "World" true))