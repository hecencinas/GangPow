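; BP_GangPowGameMode is the game mode that sets up the game's teams and their on-screen display at start.
; BeginPlay spawns two BP_Team actors at the world origin, the second set to look for characters tagged Enemy, and collects both in a Teams array.
; It then passes that array to a WBP_Teams widget for the first player controller and adds it to the viewport.
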(event EventBeginPlay
  (bind _returnvalue (Game|SpawnActorfromClass "/Game/Blueprints/BP_Team.BP_Team_C" (Math|Transform|MakeTransform "0, 0, 0") "Undefined" 0 "Player" 0))
  (Utilities|Array|Add (Variables|Default|GetTeams) _returnvalue)
  (bind _returnvalue_2 (Game|SpawnActorfromClass "/Game/Blueprints/BP_Team.BP_Team_C" (Math|Transform|MakeTransform "0, 0, 0") "Undefined" 0 "Enemy" 0))
  (Utilities|Array|Add (Variables|Default|GetTeams) _returnvalue_2)
  (bind _returnvalue_3 (UserInterface|CreateWidget "/Game/Blueprints/WBP_Teams.WBP_Teams_C" (Game|GetPlayerController 0) (Variables|Default|GetTeams)))
  (UserInterface|Viewport|AddtoViewport _returnvalue_3 0))

(event EventTick
  (params (DeltaSeconds :type Float%20%28single-precision%29)))

(fn ConstructionScript)