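; BP_PlayerCharacter is the player character, holding its health and a set of action components.
; BeginPlay fills HP and adds a component for each initial action class, which can be looked up by action type or queried for the hand's unique widget classes.
; ReceiveDamage clamps HP, updates the health bar and broadcasts the change; a self-bound death check destroys the character at zero, and destruction empties the bar.
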(event Custom|OnDestroy
  (params (DestroyedActor :type Actor%20Object%20Reference))
  (if (== DestroyedActor self)
    (Progress|SetPercent (Variables|Default|GetHealthBar) 0.0)))

(event Custom|DeathCheck
  (params (Character :type BP%20Player%20Character%20Object%20Reference) (NewHealth :type Float%20%28single-precision%29) (MaxHealth :type Float%20%28single-precision%29))
  (if (<= NewHealth 0.0)
    (Utilities|IsValid Character
      (:Is%20Valid
        (Actor|DestroyActor Character)))))

(event EventBeginPlay
  (EventDispatchers|BindEventtoNotifyHealthChanged (EventDispatchers|CreateEvent :!event Custom|DeathCheck))
  (Game|BindEventtoOnDestroyed (EventDispatchers|CreateEvent :!event Custom|OnDestroy))
  (Variables|Default|SetHP (Variables|Default|GetMaxHP))
  (for _array_element (Variables|Default|GetInitialActionsClasses)
    (bind _returnvalue (Game|AddComponentbyClass _array_element))
    (Utilities|Array|Add (Variables|Default|GetAvailableActions) _returnvalue)))

(fn ConstructionScript)

(fn GetCharacterHand
  (for _array_element (Variables|Default|GetAvailableActions)
    (Utilities|Array|AddUnique (LocalVariables|GetCharacterActionClasses) (Default|GetActionWidgetClass _array_element)))
  (return (LocalVariables|GetCharacterActionClasses)))

(fn GetCurHp
  (return (Variables|Default|GetHP)))

(fn GetMaxHp
  (return (Variables|Default|GetMaxHP)))

(fn ReceiveDamage
  (params (B :type Float%20%28single-precision%29))
  (bind _self self)
  (bind _maxhp (Variables|Default|GetMaxHP))
  (bind _output_get (Variables|Default|SetHP (Math|Float|Clamp(Float) (- (Variables|Default|GetHP) B) 0.0 (Variables|Default|GetMaxHP))))
  (Progress|SetPercent (Variables|Default|GetHealthBar) (/ _output_get _maxhp))
  (Default|CallNotifyHealthChanged _self _self _output_get _maxhp))

(fn GetAction
  (params (ActionType :type EActions%20Enum :default "NewEnumerator0"))
  (for _array_element (Variables|Default|GetAvailableActions)
    (if (Utilities|Enum|Equal(Enum) (Default|GetActionType _array_element) ActionType)
      (return _array_element)))
  (return 0))