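; Actor component that lets the player aim a shot by drawing an arrow on screen, previewing the predicted projectile path.
; Arrow widget updates set the owner's yaw and launch velocity from the drawn angle and length.
; A projectile path trace then fills a runtime spline with an attached Niagara effect.
; Ending the draw executes the GameState's selected action with the owner's AI controller; enable and disable toggle preview and input mode.
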(event EventBeginPlay
  (bind _returnvalue (Game|AddComponentbyClass (Components|GetOwner) "/Script/Engine.SplineComponent" false))
  (bind _output_get (Variables|Default|SetSpline _returnvalue))
  (Spline|SetSplinePoints _output_get (Utilities|Array|MakeArray) "Local" true)
  (Niagara|SpawnSystemAttached "/Game/Blueprints/NS_ProjectilePath.NS_ProjectilePath" _output_get "None" "0, 0, 0" "0, 0, 0" "SnapToTarget" false true "AutoRelease")
  (bind _returnvalue_2 (UserInterface|CreateWidget "/Game/Blueprints/WBP_ArrowDraw.WBP_ArrowDraw_C" (Game|GetPlayerController 0)))
  (bind _output_get_2 (Variables|Default|SetArrowWidget _returnvalue_2))
  (UserInterface|Viewport|AddtoViewport _output_get_2 0)
  (Input|SetInputModeUIOnly (Game|GetPlayerController 0) 0 "LockAlways")
  (EventDispatchers|BindEventtoNotifyDrawEnded (Variables|Default|GetArrowWidget) (EventDispatchers|CreateEvent :!event OnArrowDrawNotifyEnd))
  (EventDispatchers|BindEventtoNotifyArrowDrawUpdate (Variables|Default|GetArrowWidget) (EventDispatchers|CreateEvent :!event OnArrowDrawNotifyUpdate)))

(event EventTick
  (params (DeltaSeconds :type Float%20%28single-precision%29)))

(event EventDisable
  (CallFunction|DisablePrediction))

(event EventEnable
  (CallFunction|EnablePrediction))

(fn UpdateShootPreview
  (Transformation|SetActorRotation (Components|GetOwner) (Math|Rotator|MakeRotator 0.0 0.0 (+ (Variables|/Game/Blueprints/WBP_ArrowDraw.WBP_ArrowDraw_C|GetCurAngle (Variables|Default|GetArrowWidget)) 9e+01)))
  (bind _output_get (Variables|Default|SetLastVelocity (* (Transformation|GetActorForwardVector (Components|GetOwner)) (* 750 (Variables|/Game/Blueprints/WBP_ArrowDraw.WBP_ArrowDraw_C|GetCurVectorLength (Variables|Default|GetArrowWidget))))))
  (bind _outpathpositions (Class|GameplayStatics|BlueprintPredictProjectilePathbyTraceChannel (Transformation|GetActorLocation (Components|GetOwner)) _output_get true 1.0 "ECC_Visibility" false (Utilities|Array|MakeArray (Components|GetOwner)) "None"))
  (Spline|SetSplinePoints (Variables|Default|GetSpline) _outpathpositions "World" true))

(fn EnablePrediction
  (Variables|Default|SetEnabled true)
  (Class|IPlayerComponentsInterface|Enable(Message) (Variables|Default|GetArrowWidget))
  (Input|SetInputModeUIOnly (Game|GetPlayerController 0) 0 "LockAlways"))

(fn DisablePrediction
  (Variables|Default|SetEnabled false)
  (Spline|SetSplinePoints (Variables|Default|GetSpline) (Utilities|Array|MakeArray) "World" true)
  (Class|IPlayerComponentsInterface|Disable(Message) (Variables|Default|GetArrowWidget))
  (Input|SetInputModeGameandUI (Game|GetPlayerController 0) 0 "LockAlways" false))

(fn OnArrowDrawNotifyUpdate
  (if (Variables|Default|GetEnabled)
    (CallFunction|UpdateShootPreview)))

(fn OnArrowDrawNotifyEnd
  (Default|Execute (Variables|/Game/Blueprints/BP_GameStateBase.BP_GameStateBase_C|GetSelectedAction (.AsBP%20Game%20State%20Base (Utilities|Casting|CastToBP_GameStateBase (Game|GetGameState)))) (AI|GetAIController (Components|GetOwner))))