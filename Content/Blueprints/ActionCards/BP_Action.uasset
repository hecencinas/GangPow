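; BP_Action is a base for action-card actions, each exposing an action type and a card widget class.
; It binds to game-state changes, disabling the selected player character's preview during character selection and enabling it when a matching action type is being played.
; Preview functions for players and enemies are empty stubs, apparently for child overrides.
; Both Execute functions only inform the game state that the action executed.
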(event Custom|OnGameStateChange
  (bind _game_state (Variables|Default|GetGame%20State))
  (bind _selectedcharacter (Default|GetCurrentlySelectedCharacter _game_state))
  (bind _returnvalue (AI|GetAIController _selectedcharacter))
  (bind (_asaic_player_character _bsuccess) (Utilities|Casting|CastToAIC_PlayerCharacter _returnvalue))
  (switch Utilities|FlowControl|Switch|SwitchonEGameState (Default|GetCurrentlyGameState _game_state)
    (:NewEnumerator0
      (if true
        (CallFunction|DisablePreviewforPlayer _asaic_player_character)))
    (:NewEnumerator2
      (if (and (Utilities|Enum|Equal(Enum) (Default|GetCurrentlySelectedActionType _game_state) (Variables|Default|GetActionType)) _bsuccess)
        (CallFunction|EnablePreviewforPlayer _asaic_player_character)))))

(event EventBeginPlay
  (bind _output_get (Variables|Default|SetGame%20State (.AsBP%20Game%20State%20Base (Utilities|Casting|CastToBP_GameStateBase (Game|GetGameState)))))
  (EventDispatchers|BindEventtoChangedGameState _output_get (EventDispatchers|CreateEvent :!event Custom|OnGameStateChange)))

(fn ExecuteforPlayer
  (params (TargetController :type AIC%20Player%20Character%20Object%20Reference))
  (Default|InformActionExecuted (Variables|Default|GetGame%20State) self))

(fn EnablePreviewforPlayer
  (params (TargetController :type AIC%20Player%20Character%20Object%20Reference)))

(fn DisablePreviewforPlayer
  (params (TargetController :type AIC%20Player%20Character%20Object%20Reference)))

(fn GetActionWidgetClass
  (return (Variables|Default|GetActionCardClass)))

(fn GetActionType
  (return (Variables|Default|GetActionType)))

(fn ExecuteforEnemy
  (params (TargetController :type AIC%20Player%20Character%20Object%20Reference))
  (Default|InformActionExecuted (Variables|Default|GetGame%20State) self))

(fn EnablePreviewforEnemy
  (params (TargetController :type AIC%20Player%20Character%20Object%20Reference)))

(fn DisablePreviewforEnemy
  (params (TargetController :type AIC%20Player%20Character%20Object%20Reference)))