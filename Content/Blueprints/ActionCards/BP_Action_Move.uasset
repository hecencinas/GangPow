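; BP_Action_Move is the move action card, overriding the execute and preview steps of its parent action.
; Executing selects its action type on the GameState, sends a try-move message to the target controller, and runs parent logic only if that succeeds.
; Preview toggles call the parent, then send the controller predict-shoot enable or disable messages with the player prediction component class, reusing shoot-named messages for movement.
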(event EventBeginPlay
  (|CallParentFunction) ; This node is disabled and will not be called.\nDrag off pins to build functionality.
)

(event EventTick
  (params (DeltaSeconds :type Float%20%28single-precision%29)))

(fn ExecuteforPlayer
  (params (TargetController :type AIC%20Player%20Character%20Object%20Reference))
  (Default|SelectAction (Variables|Default|GetGame%20State) (CallFunction|GetActionType))
  (bind _success (Class|IAIActions|AITryMoveto(Message) TargetController))
  (if _success
    (|CallParentFunction TargetController)))

(fn EnablePreviewforPlayer
  (params (TargetController :type AIC%20Player%20Character%20Object%20Reference))
  (|CallParentFunction TargetController)
  (Class|IAIActions|AIPredictShoot(Message) TargetController (Variables|Default|GetPrediction%20Comp%20Class%20For%20Player)))

(fn DisablePreviewforPlayer
  (params (TargetController :type AIC%20Player%20Character%20Object%20Reference))
  (|CallParentFunction TargetController)
  (Class|IAIActions|AIDisablePredictShoot(Message) TargetController (Variables|Default|GetPrediction%20Comp%20Class%20For%20Player)))