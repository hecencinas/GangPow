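; Jump action card that launches the target controller's pawn along a previewed jump.
; Preview enable and disable call the parent, then tell the controller to start or stop prediction with the card's prediction component class.
; Execution fetches that component as BPC_PredictJump, launches the Character with its LastVelocity and disables it.
; The parent execute runs afterwards regardless of whether the launch succeeds.
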(event EventBeginPlay
  (|CallParentFunction) ; This node is disabled and will not be called.\nDrag off pins to build functionality.
)

(event EventTick
  (params (DeltaSeconds :type Float%20%28single-precision%29)))

(fn ExecuteforPlayer
  (params (TargetController :type AIC%20Player%20Character%20Object%20Reference))
  (bind _value (Default|GetPredictionComp TargetController (Variables|Default|GetPrediction%20Comp%20Class%20For%20Player)))
  (CallFunction|Shoot (Pawn|GetControlledPawn TargetController) _value)
  (if true
    (|CallParentFunction TargetController)))

(fn EnablePreviewforPlayer
  (params (TargetController :type AIC%20Player%20Character%20Object%20Reference))
  (|CallParentFunction TargetController)
  (Class|IAIActions|AIPredictShoot(Message) TargetController (Variables|Default|GetPrediction%20Comp%20Class%20For%20Player)))

(fn DisablePreviewforPlayer
  (params (TargetController :type AIC%20Player%20Character%20Object%20Reference))
  (|CallParentFunction TargetController)
  (Class|IAIActions|AIDisablePredictShoot(Message) TargetController (Variables|Default|GetPrediction%20Comp%20Class%20For%20Player)))

(fn Shoot
  (params (Owner :type Actor%20Object%20Reference) (PredictionComp :type Object%20Object%20Reference))
  (LocalVariables|SetpOwner Owner)
  (bind _asbpc_predict_jump (Utilities|Casting|CastToBPC_PredictJump PredictionComp)
    (:then
      (LocalVariables|SetpPredictionComp _asbpc_predict_jump)
      (bind _ascharacter (Utilities|Casting|CastToCharacter (LocalVariables|GetpOwner))
        (:then
          (Character|LaunchCharacter _ascharacter (Variables|/Game/Blueprints/PredictionComponents/BPC_PredictJump.BPC_PredictJump_C|GetLastVelocity _asbpc_predict_jump) false false)
          (Default|Disable (LocalVariables|GetpPredictionComp))
          (return true))
        (:CastFailed
          _)))
    (:CastFailed
      _))
  (return false))