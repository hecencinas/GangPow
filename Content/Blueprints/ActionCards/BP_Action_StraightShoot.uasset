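; Action card that fires a straight-shot projectile from the player's pawn, with an aim preview driven through the controller's prediction component.
; Preview enable and disable send predict-shoot messages to the controller, while enemy previews only call the parent.
; Shoot launches a BP_BasicProjectile using the arrow-draw predictor's last velocity, or falls back to a suggested arc toward the cursor hit.
; The parent execute runs only if the shot succeeds.
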(event EventBeginPlay
  (|CallParentFunction) ; This node is disabled and will not be called.\nDrag off pins to build functionality.
)

(event EventTick
  (params (DeltaSeconds :type Float%20%28single-precision%29)))

(fn ExecuteforPlayer
  (params (TargetController :type AIC%20Player%20Character%20Object%20Reference))
  (bind _value (Default|GetPredictionComp TargetController (Variables|Default|GetPrediction%20Comp%20Class%20For%20Player)))
  (bind _success (CallFunction|Shoot (Pawn|GetControlledPawn TargetController) _value))
  (if _success
    (|CallParentFunction TargetController)))

(fn EnablePreviewforPlayer
  (params (TargetController :type AIC%20Player%20Character%20Object%20Reference))
  (|CallParentFunction TargetController)
  (Class|IAIActions|AIPredictShoot(Message) TargetController (Variables|Default|GetPrediction%20Comp%20Class%20For%20Player)))

(fn DisablePreviewforPlayer
  (params (TargetController :type AIC%20Player%20Character%20Object%20Reference))
  (|CallParentFunction TargetController)
  (Class|IAIActions|AIDisablePredictShoot(Message) TargetController (Variables|Default|GetPrediction%20Comp%20Class%20For%20Player)))

(fn Shoot
  (params (Owner :type Actor%20Object%20Reference) (PredictionComp :type Object%20Object%20Reference))
  (bind _returnvalue (Game|GetPlayerController 0))
  (bind _array (Utilities|Array|MakeArray "ObjectTypeQuery7" "ObjectTypeQuery1"))
  (bind (_hitresult _returnvalue_2) (Class|PlayerController|GetHitResultUnderCursorforObjects _returnvalue _array true))
  (LocalVariables|SetpOwner Owner)
  (bind _asbpc_predict_shoot_with_arrow_draw (Utilities|Casting|CastToBPC_PredictShootWithArrowDraw PredictionComp)
    (:then
      (LocalVariables|SetpPredictionComp _asbpc_predict_shoot_with_arrow_draw)
      (bind _returnvalue_3 (Game|SpawnActorfromClass "/Game/Blueprints/BP_BasicProjectile.BP_BasicProjectile_C" (Math|Transform|MakeTransform (.location (Transformation|GetActorTransform (LocalVariables|GetpOwner))) "0, 0, 0" "1,1,1") "AlwaysSpawn" (LocalVariables|GetpOwner) 0))
      (Components|Activation|Activate (Variables|/Game/Blueprints/BP_BasicProjectile.BP_BasicProjectile_C|GetProjectileMovement _returnvalue_3) true)
      (Game|Components|ProjectileMovement|SetVelocityinLocalSpace (Variables|/Game/Blueprints/BP_BasicProjectile.BP_BasicProjectile_C|GetProjectileMovement _returnvalue_3) (Variables|/Game/Blueprints/PredictionComponents/BPC_PredictShootWithArrowDraw.BPC_PredictShootWithArrowDraw_C|GetLastVelocity (LocalVariables|GetpPredictionComp)))
      (Default|Disable (LocalVariables|GetpPredictionComp))
      (return true))
    (:CastFailed
      (if _returnvalue_2
        (bind _outlaunchvelocity (Game|SuggestProjectileVelocityCustomArc (Transformation|GetActorLocation (LocalVariables|GetpOwner)) (.impactpoint _hitresult) 0.0 0.5))
        (bind _returnvalue_4 (Game|SpawnActorfromClass "/Game/Blueprints/BP_BasicProjectile.BP_BasicProjectile_C" (Math|Transform|MakeTransform (+ (.location (Transformation|GetActorTransform (LocalVariables|GetpOwner))) (* (Transformation|GetActorForwardVector (LocalVariables|GetpOwner)) 5.0)) "0, 0, 0" "1,1,1") "AlwaysSpawn" (LocalVariables|GetpOwner) 0))
        (Components|Activation|Activate (Variables|/Game/Blueprints/BP_BasicProjectile.BP_BasicProjectile_C|GetProjectileMovement _returnvalue_4) true)
        (Game|Components|ProjectileMovement|SetVelocityinLocalSpace (Variables|/Game/Blueprints/BP_BasicProjectile.BP_BasicProjectile_C|GetProjectileMovement _returnvalue_4) _outlaunchvelocity)
        (return true)
        (else
          (return false))))))

(fn DisablePreviewforEnemy
  (params (TargetController :type AIC%20Player%20Character%20Object%20Reference))
  (|CallParentFunction 0))

(fn EnablePreviewforEnemy
  (params (TargetController :type AIC%20Player%20Character%20Object%20Reference))
  (|CallParentFunction 0))