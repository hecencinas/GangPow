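; BP_Action_CurvedShoot is an action card that fires a projectile along a predicted curved trajectory from the player's pawn.
; Enabling or disabling preview messages the controller to show or hide the prediction component.
; Execution spawns BP_BasicProjectile with the last velocity from BPC_PredictCurvedShootWithVelocity, then disables that component.
; The parent execute logic runs only if the component cast succeeds and the shot fires.
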(event EventBeginPlay
  (|CallParentFunction) ; This node is disabled and will not be called.\nDrag off pins to build functionality.
)

(event EventTick
  (params (DeltaSeconds :type Float%20%28single-precision%29)))

(fn ExecuteforPlayer
  (params (TargetController :type AIC%20Player%20Character%20Object%20Reference))
  (bind _value (Default|GetPredictionComp TargetController (Variables|Default|GetPrediction%20Comp%20Class%20For%20Player)))
  (bind _success (CallFunction|Shoot (Pawn|GetControlledPawn TargetController) _value))
  (if _success
    (|CallParentFunction TargetController)))

(fn EnablePreviewforPlayer
  (params (TargetController :type AIC%20Player%20Character%20Object%20Reference))
  (|CallParentFunction TargetController)
  (Class|IAIActions|AIPredictShoot(Message) TargetController (Variables|Default|GetPrediction%20Comp%20Class%20For%20Player)))

(fn DisablePreviewforPlayer
  (params (TargetController :type AIC%20Player%20Character%20Object%20Reference))
  (|CallParentFunction TargetController)
  (Class|IAIActions|AIDisablePredictShoot(Message) TargetController (Variables|Default|GetPrediction%20Comp%20Class%20For%20Player)))

(fn Shoot
  (params (Owner :type Actor%20Object%20Reference) (PredictionComp :type Object%20Object%20Reference))
  (LocalVariables|SetpOwner Owner)
  (bind _asbpc_predict_curved_shoot_with_velocity (Utilities|Casting|CastToBPC_PredictCurvedShootWithVelocity PredictionComp)
    (:then
      (LocalVariables|SetpPredictionComp _asbpc_predict_curved_shoot_with_velocity)
      (bind _returnvalue (Game|SpawnActorfromClass "/Game/Blueprints/BP_BasicProjectile.BP_BasicProjectile_C" (Math|Transform|MakeTransform (.location (Transformation|GetActorTransform (LocalVariables|GetpOwner))) "0, 0, 0" "1,1,1") "AlwaysSpawn" (LocalVariables|GetpOwner) 0))
      (Components|Activation|Activate (Variables|/Game/Blueprints/BP_BasicProjectile.BP_BasicProjectile_C|GetProjectileMovement _returnvalue) true)
      (Game|Components|ProjectileMovement|SetVelocityinLocalSpace (Variables|/Game/Blueprints/BP_BasicProjectile.BP_BasicProjectile_C|GetProjectileMovement _returnvalue) (Variables|/Game/Blueprints/PredictionComponents/BPC_PredictCurvedShootWithVelocity.BPC_PredictCurvedShootWithVelocity_C|GetLastVelocity (LocalVariables|GetpPredictionComp)))
      (Default|Disable (LocalVariables|GetpPredictionComp))
      (return true))
    (:CastFailed
      (return false))))