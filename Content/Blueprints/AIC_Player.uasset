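; AI controller for a player-side pawn that handles move-to-cursor and shot prediction requests.
; Prediction components are added to the pawn on first use, cached by class in a map, then enabled, disabled or looked up through it.
; Movement sends the pawn to the visibility-trace hit under player 0's cursor.
; AI Shoot At only returns true; its projectile code is unreachable, with a note that shooting moved to the card implementation.
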(event EventBeginPlay)

(event EventTick
  (params (DeltaSeconds :type Float%20%28single-precision%29)))

(fn ConstructionScript)

(fn GetPredictionComp
  (params (PredictionCompClass :type Base%20BPC%20Prediction%20Component%20Class%20Reference))
  (bind _spawnedpredictioncomps (Variables|Default|GetSpawnedPredictionComps))
  (bind (_value _returnvalue) (Utilities|Map|Find _spawnedpredictioncomps PredictionCompClass))
  (if _returnvalue
    (return _value)
    (else
      (return 0))))

(fn AIDisablePredictShoot
  (params (PredictionCompClass :type Base%20BPC%20Prediction%20Component%20Class%20Reference))
  (LocalVariables|SetpPredictionCompClass PredictionCompClass)
  (if (.ReturnValue (Utilities|Map|Find (Variables|Default|GetSpawnedPredictionComps) (LocalVariables|GetpPredictionCompClass)))
    (Default|Disable (.Value (Utilities|Map|Find (Variables|Default|GetSpawnedPredictionComps) (LocalVariables|GetpPredictionCompClass))))
    (return true)
    (else
      (return true))))

(fn AIPredictShoot
  (params (PredictionCompClass :type Base%20BPC%20Prediction%20Component%20Class%20Reference))
  (LocalVariables|SetpPredictionCompClass PredictionCompClass)
  (if (.ReturnValue (Utilities|Map|Find (Variables|Default|GetSpawnedPredictionComps) (LocalVariables|GetpPredictionCompClass)))
    (bind _output_get (LocalVariables|SetUsingPredictionComp (.Value (Utilities|Map|Find (Variables|Default|GetSpawnedPredictionComps) (LocalVariables|GetpPredictionCompClass)))))
    (Utilities|IsValid _output_get
      (:Is%20Valid
        _)
      (:Is%20Not%20Valid
        (bind _returnvalue (Game|AddComponentbyClass (Pawn|GetControlledPawn) (LocalVariables|GetpPredictionCompClass) :!label _label))
        (Utilities|Map|Add (Variables|Default|GetSpawnedPredictionComps) (LocalVariables|GetpPredictionCompClass) _returnvalue)
        (LocalVariables|SetUsingPredictionComp _returnvalue)))
    (else
      (goto _label)))
  (Default|Enable (LocalVariables|GetUsingPredictionComp))
  (return true))

(fn AIShootat
  (params (PredictionCompClass :type Base%20BPC%20Prediction%20Component%20Class%20Reference))
  (return true))

(fn AITryMoveto
  (bind _returnvalue (Game|GetPlayerController 0))
  (bind (_hitresult _returnvalue_2) (Game|Player|GetHitResultUnderCursorbyChannel _returnvalue "TraceTypeQuery1" true))
  (if _returnvalue_2
    (AI|Navigation|MovetoLocation (.impactpoint _hitresult) -1.0 true true false true 0))
  (return _returnvalue_2))