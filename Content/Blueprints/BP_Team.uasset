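; BP_Team is an actor that tracks a team of characters placed in the level.
; On BeginPlay it gathers every actor with a configurable tag into TeamCharacters, with no later refresh in this Blueprint.
; Accessor functions return the whole list or the member at a given index cast to BP_PlayerCharacter.
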(event EventBeginPlay
  (bind _outactors (Actor|GetAllActorswithTag (Variables|Default|GetLookingForCharacterTag)))
  (Variables|Default|SetTeamCharacters _outactors))

(event Collision|EventActorBeginOverlap
  (params (OtherActor :type Actor%20Object%20Reference)))

(event EventTick
  (params (DeltaSeconds :type Float%20%28single-precision%29)))

(fn ConstructionScript)

(fn GetTeamMembers
  (return (Variables|Default|GetTeamCharacters)))

(fn GetPlayerCharacter
  (params (Index :type Integer))
  (bind _asbp_player_character (Utilities|Casting|CastToBP_PlayerCharacter (Utilities|Array|Get(acopy) (Variables|Default|GetTeamCharacters) Index))
    (:then
      (return _asbp_player_character))
    (:CastFailed
      (return 0))))