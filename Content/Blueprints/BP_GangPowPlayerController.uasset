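; Player controller that turns the Select input into character selection or action execution, depending on the current game state.
; While selecting a character, a cursor trace finds a Player-tagged character and passes it to the game state.
; While playing an action, it executes the selected character's chosen action through that character's AI controller.
; Arrow-drawing widget setup with UI-only input exists but is unconnected and never runs.
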(event EventBeginPlay)

(event Input|ActionEvents|InputActionSelect
  (params (Key :type Key%20Structure))
  (:Pressed
    (Utilities|IsValid (Variables|Default|GetGame%20State)
      (:Is%20Valid
        _)
      (:Is%20Not%20Valid
        (Variables|Default|SetGame%20State (.AsBP%20Game%20State%20Base (Utilities|Casting|CastToBP_GameStateBase (Game|GetGameState))))))
    (switch Utilities|FlowControl|Switch|SwitchonEGameState (Default|GetCurrentlyGameState (Variables|Default|GetGame%20State))
      (:NewEnumerator0
        (bind _asbp_player_character (Utilities|Casting|CastToBP_PlayerCharacter (.hitactor (.HitResult (Class|PlayerController|GetHitResultUnderCursorforObjects (Utilities|Array|MakeArray "ObjectTypeQuery7") true)))))
        (if (>= (Utilities|Array|FindItem (Variables|/Script/Engine.Actor|GetTags _asbp_player_character) "Player") 0)
          (Default|SelectCharacter (Variables|Default|GetGame%20State) _asbp_player_character)))
      (:NewEnumerator2
        (bind _asaic_player_character (Utilities|Casting|CastToAIC_PlayerCharacter (AI|GetAIController (Variables|/Game/Blueprints/BP_GameStateBase.BP_GameStateBase_C|GetSelectedCharacter (Variables|Default|GetGame%20State)))))
        (Default|ExecuteforPlayer (Default|GetAction (Variables|/Game/Blueprints/BP_GameStateBase.BP_GameStateBase_C|GetSelectedCharacter (Variables|Default|GetGame%20State)) (Variables|/Game/Blueprints/BP_GameStateBase.BP_GameStateBase_C|GetSelectedAction (Variables|Default|GetGame%20State))) _asaic_player_character)))))

(fn ConstructionScript)