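; Game state Blueprint that runs a three-stage selection flow: pick a character, pick an action, then await its execution.
; Each selection is accepted only in its matching enum state, then advances the state and fires a changed-state dispatcher.
; Selecting an action enables its preview on the character's AI controller; reporting execution disables it and resets the flow.
; BeginPlay also creates the in-game HUD for the first player.
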(event EventBeginPlay
  (bind _returnvalue (UserInterface|CreateWidget "/Game/Blueprints/WBP_InGameHUD.WBP_InGameHUD_C" (Game|GetPlayerController 0)))
  (bind _output_get (Variables|Default|SetInGameHUD _returnvalue))
  (UserInterface|Viewport|AddtoViewport _output_get 0))

(event EventTick
  (params (DeltaSeconds :type Float%20%28single-precision%29)))

(fn ConstructionScript)

(fn GetCurrentGameState
  (return (Variables|Default|GetCurrentState)))

(fn SelectCharacter
  (params (SelectedCharacter :type BP%20Player%20Character%20Object%20Reference))
  (if (Utilities|Enum|Equal(Enum) (Variables|Default|GetCurrentState) "NewEnumerator0")
    (Variables|Default|SetSelectedCharacter SelectedCharacter)
    (Variables|Default|SetCurrentState "NewEnumerator1")
    (Default|CallChangedGameState)))

(fn SelectAction
  (params (SelectedAction :type WBP%20Action%20Card%20Object%20Reference))
  (if (Utilities|Enum|Equal(Enum) (Variables|Default|GetCurrentState) "NewEnumerator1")
    (bind _output_get (Variables|Default|SetSelectedAction SelectedAction))
    (Variables|Default|SetCurrentState "NewEnumerator2")
    (Default|EnablePreview _output_get (AI|GetAIController (Variables|Default|GetSelectedCharacter)))
    (Default|CallChangedGameState)))

(fn InformActionExecuted
  (params (ActionPlayed :type WBP%20Action%20Card%20Object%20Reference))
  (Default|DisablePreview ActionPlayed (AI|GetAIController (Variables|Default|GetSelectedCharacter)))
  (Variables|Default|SetCurrentState "NewEnumerator0")
  (Default|CallChangedGameState))