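; Melee strike prediction component that previews how struck player characters get launched while the player aims with a drag-arrow widget.
; Arrow angle rotates the owner and length scales launch velocity; a short box trace along negative forward finds targets.
; Each target's predicted projectile path feeds its own spline preview component, and dropped targets are cleared.
; Ending the draw executes the selected action if the owner is the selected character.
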(event EventBeginPlay
  (for _array_element (Actor|GetComponentsByClass (Components|GetOwner) "/Script/Engine.SplineComponent")
    (Utilities|IsValid _array_element
      (:Is%20Valid
        (Utilities|Array|AddUnique (Variables|Default|GetSplines) _array_element)
        (Spline|SetSplinePoints _array_element (Utilities|Array|MakeArray) "Local" true))))
  (bind _returnvalue (UserInterface|CreateWidget "/Game/Blueprints/PredictionComponents/WBP_ArrowDrawForPlayer.WBP_ArrowDrawForPlayer_C" (Game|GetPlayerController 0)))
  (bind _output_get (Variables|Default|SetArrowWidget _returnvalue))
  (UserInterface|Viewport|AddtoViewport _output_get 0)
  (Input|SetInputModeUIOnly (Game|GetPlayerController 0) 0 "LockAlways")
  (EventDispatchers|BindEventtoNotifyDrawEnded (Variables|Default|GetArrowWidget) (EventDispatchers|CreateEvent :!event OnArrowDrawNotifyEnd))
  (EventDispatchers|BindEventtoNotifyArrowDrawUpdate (Variables|Default|GetArrowWidget) (EventDispatchers|CreateEvent :!event OnArrowDrawNotifyUpdate)))

(fn UpdateShootPreview
  (bind _returnvalue (Components|GetOwner))
  (bind _characterspredicting (Variables|Default|GetCharactersPredicting))
  (bind _returnvalue_2 (Transformation|GetActorLocation _returnvalue))
  (LocalVariables|SetLastSplineUsed 0)
  (Transformation|SetActorRotation (Components|GetOwner) (Math|Rotator|MakeRotator 0.0 0.0 (Variables|/Game/Blueprints/PredictionComponents/WBP_ArrowDrawForPlayer.WBP_ArrowDrawForPlayer_C|GetCurAngle (Variables|Default|GetArrowWidget))))
  (Variables|Default|SetLastVelocity (* (+ (Transformation|GetActorForwardVector (Components|GetOwner)) "0, 0,-0.200000") (* 300 (Variables|/Game/Blueprints/PredictionComponents/WBP_ArrowDrawForPlayer.WBP_ArrowDrawForPlayer_C|GetCurVectorLength (Variables|Default|GetArrowWidget)))))
  (bind _keys (Utilities|Map|Keys _characterspredicting))
  (for _array_element _keys
    (Utilities|Map|Add _characterspredicting _array_element false))
  (bind (_outhits _returnvalue_3) (Class|KismetSystemLibrary|BoxTraceMultiforObjects _returnvalue_2 (+ _returnvalue_2 (* (Transformation|GetActorForwardVector (Components|GetOwner)) -6e+01)) "0,30.000000,30.000000" (Transformation|GetActorRotation _returnvalue) (Utilities|Array|MakeArray "ObjectTypeQuery7") false (Utilities|Array|MakeArray _returnvalue) "ForOneFrame" true))
  (if _returnvalue_3
    (for _array_element_2 _outhits
      (bind _asbp_player_character (Utilities|Casting|CastToBP_PlayerCharacter (.hitactor _array_element_2)))
      (LocalVariables|SetUpdatingCharacter _asbp_player_character)
      (Utilities|Map|Add (Variables|Default|GetCharactersPredicting) _asbp_player_character true)
      (if (< (Utilities|Array|Length (Variables|Default|GetSplines)) (LocalVariables|GetLastSplineUsed))
        _
        (else
          (bind _returnvalue_4 (Game|AddComponentbyClass (Components|GetOwner) "/Script/Engine.SplineComponent" false))
          (Spline|SetSplinePoints _returnvalue_4 (Utilities|Array|MakeArray) "Local" true)
          (bind _returnvalue_5 (Utilities|Array|Add (Variables|Default|GetSplines) _returnvalue_4))
          (LocalVariables|SetLastSplineUsed _returnvalue_5)))
      (bind _outpathpositions (Class|GameplayStatics|BlueprintPredictProjectilePathbyTraceChannel (Transformation|GetActorLocation (LocalVariables|GetUpdatingCharacter)) (Variables|Default|GetLastVelocity) true 1.0 "ECC_Visibility" false (Utilities|Array|MakeArray (LocalVariables|GetUpdatingCharacter)) "None"))
      (Default|UpdateShootPreview (Variables|/Game/Blueprints/BP_PlayerCharacter.BP_PlayerCharacter_C|GetBPC_PredictShootWithReceivedSpline (LocalVariables|GetUpdatingCharacter)) _outpathpositions)))
  (bind _keys_2 (Utilities|Map|Keys (Variables|Default|GetCharactersPredicting)))
  (for _array_element_3 _keys_2
    (if (not (.Value (Utilities|Map|Find (Variables|Default|GetCharactersPredicting) _array_element_3)))
      (Default|DisablePrediction (Variables|/Game/Blueprints/BP_PlayerCharacter.BP_PlayerCharacter_C|GetBPC_PredictShootWithReceivedSpline _array_element_3))
      (Utilities|Map|Remove (Variables|Default|GetCharactersPredicting) _array_element_3)))
  (LocalVariables|SetUpdatingCharacter 0))

(fn EnablePrediction
  (Default|Enable (Variables|Default|GetArrowWidget))
  (Input|SetInputModeUIOnly (Game|GetPlayerController 0) 0 "LockAlways"))

(fn DisablePrediction
  (bind _keys (Utilities|Map|Keys (Variables|Default|GetCharactersPredicting)))
  (for _array_element _keys
    (Default|DisablePrediction (Variables|/Game/Blueprints/BP_PlayerCharacter.BP_PlayerCharacter_C|GetBPC_PredictShootWithReceivedSpline _array_element))
    (Utilities|Map|Remove (Variables|Default|GetCharactersPredicting) _array_element))
  (Default|Disable (Variables|Default|GetArrowWidget))
  (Input|SetInputModeGameandUI (Game|GetPlayerController 0) 0 "LockAlways" false))

(fn OnArrowDrawNotifyUpdate
  (if (Variables|Default|GetEnabled)
    (CallFunction|UpdateShootPreview)))

(fn OnArrowDrawNotifyEnd
  (bind _returnvalue (Game|GetGameState))
  (bind _returnvalue_2 (Components|GetOwner))
  (bind _asbp_game_state_base (Utilities|Casting|CastToBP_GameStateBase _returnvalue))
  (bind _selectedcharacter (Default|GetCurrentlySelectedCharacter _asbp_game_state_base))
  (bind _asaic_player_character (Utilities|Casting|CastToAIC_PlayerCharacter (AI|GetAIController _returnvalue_2)))
  (if (== _selectedcharacter _returnvalue_2)
    (Default|ExecuteforPlayer (Default|GetAction _selectedcharacter (Default|GetCurrentlySelectedActionType _asbp_game_state_base)) _asaic_player_character)))

(fn Enable
  (|CallParentFunction)
  (CallFunction|EnablePrediction))

(fn Disable
  (|CallParentFunction)
  (CallFunction|DisablePrediction))

(fn GetCharactersPredicting
  (bind _keys (Utilities|Map|Keys (Variables|Default|GetCharactersPredicting)))
  (for _array_element _keys
    (if (.Value (Utilities|Map|Find (Variables|Default|GetCharactersPredicting) _array_element))
      (Utilities|Array|Add (LocalVariables|GetRetCharactersPredicting) _array_element)))
  (return (LocalVariables|GetRetCharactersPredicting)))