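; Prediction component that lets the player aim a shot by drawing an on-screen arrow and previews the projectile path.
; Arrow widget updates rotate the owner's yaw and set launch velocity from arrow angle and length.
; The predicted trajectory fills a spline carrying an attached Niagara path effect.
; Ending the draw executes the GameState's selected action through the owner's AI controller, while Enable and Disable toggle widget and input mode.
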(event EventBeginPlay
  (bind _returnvalue (Components|GetOwner))
  (bind _returnvalue_2 (Actor|GetComponentbyClass _returnvalue "/Script/Engine.SplineComponent"))
  (Utilities|IsValid _returnvalue_2
    (:Is%20Valid
      (Variables|Default|SetSpline _returnvalue_2))
    (:Is%20Not%20Valid
      (bind _returnvalue_3 (Game|AddComponentbyClass _returnvalue "/Script/Engine.SplineComponent" false))
      (Variables|Default|SetSpline _returnvalue_3)))
  (Spline|SetSplinePoints (Variables|Default|GetSpline) (Utilities|Array|MakeArray) "Local" true)
  (bind _returnvalue_4 (Niagara|SpawnSystemAttached "/Game/Blueprints/NS_ProjectilePath.NS_ProjectilePath" (Variables|Default|GetSpline) "None" "0, 0, 0" "0, 0, 0" "SnapToTarget" false true "AutoRelease"))
  (Variables|Default|SetNiagaraSpawnedSystem _returnvalue_4)
  (bind _returnvalue_5 (UserInterface|CreateWidget "/Game/Blueprints/PredictionComponents/WBP_ArrowDraw.WBP_ArrowDraw_C" (Game|GetPlayerController 0)))
  (bind _output_get (Variables|Default|SetArrowWidget _returnvalue_5))
  (UserInterface|Viewport|AddtoViewport _output_get 0)
  (Input|SetInputModeUIOnly (Game|GetPlayerController 0) 0 "LockAlways")
  (EventDispatchers|BindEventtoNotifyDrawEnded (Variables|Default|GetArrowWidget) (EventDispatchers|CreateEvent :!event OnArrowDrawNotifyEnd))
  (EventDispatchers|BindEventtoNotifyArrowDrawUpdate (Variables|Default|GetArrowWidget) (EventDispatchers|CreateEvent :!event OnArrowDrawNotifyUpdate)))

(fn UpdateShootPreview
  (Transformation|SetActorRotation (Components|GetOwner) (Math|Rotator|MakeRotator 0.0 0.0 (Variables|/Game/Blueprints/PredictionComponents/WBP_ArrowDraw.WBP_ArrowDraw_C|GetCurAngle (Variables|Default|GetArrowWidget))))
  (bind _output_get (Variables|Default|SetLastVelocity (* (Transformation|GetActorForwardVector (Components|GetOwner)) (* 1000 (Variables|/Game/Blueprints/PredictionComponents/WBP_ArrowDraw.WBP_ArrowDraw_C|GetCurVectorLength (Variables|Default|GetArrowWidget))))))
  (bind _outpathpositions (Class|GameplayStatics|BlueprintPredictProjectilePathbyTraceChannel (Transformation|GetActorLocation (Components|GetOwner)) _output_get true 1.0 "ECC_Visibility" false (Utilities|Array|MakeArray (Components|GetOwner)) "None"))
  (Spline|SetSplinePoints (Variables|Default|GetSpline) _outpathpositions "World" true))

(fn EnablePrediction
  (Default|Enable (Variables|Default|GetArrowWidget))
  (Input|SetInputModeUIOnly (Game|GetPlayerController 0) 0 "LockAlways"))

(fn DisablePrediction
  (Spline|SetSplinePoints (Variables|Default|GetSpline) (Utilities|Array|MakeArray) "World" true)
  (Default|Disable (Variables|Default|GetArrowWidget))
  (Input|SetInputModeGameandUI (Game|GetPlayerController 0) 0 "LockAlways" false))

(fn OnArrowDrawNotifyUpdate
  (if (Variables|Default|GetEnabled)
    (CallFunction|UpdateShootPreview)))

(fn OnArrowDrawNotifyEnd
  (bind _asaic_player (Utilities|Casting|CastToAIC_Player (AI|GetAIController (Components|GetOwner))))
  (Default|Execute (Variables|/Game/Blueprints/BP_GameStateBase.BP_GameStateBase_C|GetSelectedAction (.AsBP%20Game%20State%20Base (Utilities|Casting|CastToBP_GameStateBase (Game|GetGameState)))) _asaic_player))

(fn Enable
  (|CallParentFunction)
  (CallFunction|EnablePrediction))

(fn Disable
  (|CallParentFunction)
  (CallFunction|DisablePrediction))