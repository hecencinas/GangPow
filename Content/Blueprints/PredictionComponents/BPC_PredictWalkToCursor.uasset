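; Prediction component that previews the navigation path from its owner to the point under the player's mouse cursor.
; On BeginPlay it finds or creates a spline on the owner and attaches the NS_ProjectilePath Niagara effect to it.
; While enabled, each tick traces under the cursor, fills the spline with synchronous pathfinding points raised by half the owner's world Z, and turns the owner toward the cursor.
; Disabling clears the spline.
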(event EventTick
  (params (DeltaSeconds :type Float%20%28single-precision%29))
  (if (Variables|Default|GetEnabled)
    (CallFunction|UpdateShootPreview)))

(event EventBeginPlay
  (bind _returnvalue (Components|GetOwner))
  (bind _returnvalue_2 (Actor|GetComponentbyClass _returnvalue "/Script/Engine.SplineComponent"))
  (Utilities|IsValid _returnvalue_2
    (:Is%20Valid
      (Variables|Default|SetSpline _returnvalue_2))
    (:Is%20Not%20Valid
      (bind _returnvalue_3 (Game|AddComponentbyClass _returnvalue "/Script/Engine.SplineComponent" false))
      (Variables|Default|SetSpline _returnvalue_3)))
  (Spline|SetSplinePoints (Variables|Default|GetSpline) (Utilities|Array|MakeArray) "Local" true)
  (Niagara|SpawnSystemAttached "/Game/Blueprints/NS_ProjectilePath.NS_ProjectilePath" (Variables|Default|GetSpline) "None" "0, 0, 0" "0, 0, 0" "SnapToTarget" false true "AutoRelease"))

(fn UpdateShootPreview
  (bind _returnvalue (Game|GetPlayerController 0))
  (bind _returnvalue_2 (Components|GetOwner))
  (bind _returnvalue_3 (Transformation|GetActorLocation _returnvalue_2))
  (bind (_hitresult _returnvalue_4) (Game|Player|GetHitResultUnderCursorbyChannel _returnvalue "TraceTypeQuery1" true))
  (bind (_x _y) (Math|Vector|BreakVector (.impactpoint _hitresult)))
  (if _returnvalue_4
    (bind _returnvalue_5 (Class|NavigationSystemV1|FindPathtoLocationSynchronously (Transformation|GetActorLocation (Components|GetOwner)) (.impactpoint _hitresult) 0 0))
    (bind _output_get (LocalVariables|SetNewLocalVar_0 (Variables|/Script/NavigationSystem.NavigationPath|GetPathPoints _returnvalue_5)))
    (bind _outarray (CallFunction|AddHeightonPoints _output_get))
    (Spline|SetSplinePoints (Variables|Default|GetSpline) _outarray "World" true)
    (Transformation|SetActorRotation _returnvalue_2 (Math|Rotator|FindLookatRotation (Math|Vector|MakeVector (.x _returnvalue_3) (.y _returnvalue_3) 0.0) (Math|Vector|MakeVector _x _y 0.0)))))

(fn DisablePrediction
  (Spline|SetSplinePoints (Variables|Default|GetSpline) (Utilities|Array|MakeArray) "World" true))

(fn Disable
  (|CallParentFunction)
  (CallFunction|DisablePrediction))

(fn AddHeightonPoints
  (params (InArray :type Array%20of%20Vectors))
  (for _array_element InArray
    (Utilities|Array|Add (LocalVariables|GetRetArray) (+ _array_element (Math|Vector|MakeVector 0.0 0.0 (/ (.z (Transformation|GetActorLocation (Components|GetOwner))) 2.0)))))
  (return (LocalVariables|GetRetArray)))