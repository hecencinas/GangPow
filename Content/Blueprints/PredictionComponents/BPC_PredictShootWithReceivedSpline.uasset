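; Actor component that previews a projectile's shot path along a spline fed by externally supplied points.
; On BeginPlay it reuses or adds a spline on the owner, clears it and attaches the NS_ProjectilePath Niagara system to it.
; UpdateShootPreview writes the received points to the spline in world space.
; Disabling clears the spline, while enabling only calls the parent and an empty EnablePrediction hook.
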(event EventBeginPlay
  (bind _returnvalue (Components|GetOwner))
  (bind _returnvalue_2 (Actor|GetComponentbyClass _returnvalue "/Script/Engine.SplineComponent"))
  (Utilities|IsValid _returnvalue_2
    (:Is%20Valid
      (Variables|Default|SetSpline _returnvalue_2))
    (:Is%20Not%20Valid
      (bind _returnvalue_3 (Game|AddComponentbyClass _returnvalue "/Script/Engine.SplineComponent" false))
      (Variables|Default|SetSpline _returnvalue_3)))
  (Spline|SetSplinePoints (Variables|Default|GetSpline) (Utilities|Array|MakeArray) "Local" true)
  (bind _returnvalue_4 (Niagara|SpawnSystemAttached "/Game/Blueprints/NS_ProjectilePath.NS_ProjectilePath" (Variables|Default|GetSpline) "None" "0, 0, 0" "0, 0, 0" "SnapToTarget" false true "AutoRelease"))
  (Variables|Default|SetNiagaraSpawnedSystem _returnvalue_4))

(fn UpdateShootPreview
  (params (Points :type Array%20of%20Vectors))
  (Spline|SetSplinePoints (Variables|Default|GetSpline) Points "World" true))

(fn EnablePrediction)

(fn DisablePrediction
  (Spline|SetSplinePoints (Variables|Default|GetSpline) (Utilities|Array|MakeArray) "World" true))

(fn Enable
  (|CallParentFunction)
  (CallFunction|EnablePrediction))

(fn Disable
  (|CallParentFunction)
  (CallFunction|DisablePrediction))