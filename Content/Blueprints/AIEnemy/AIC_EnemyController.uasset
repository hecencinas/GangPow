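; AI controller for the enemy side in a turn-based game, running BT_EnemyAI and mirroring the game state's enemy-turn flag into the Blackboard.
; Helper functions pick a random enemy and player target by tag, select one fixed action and preview it.
; PlayAction line-traces between Blackboard characters and, on a clear hit, launches a projectile using a suggested arc velocity.
; EndTurn is empty, and card-hand checks are disconnected.
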(event EventPossess
  (params (PossessedPawn :type Pawn%20Object%20Reference))
  (AI|RunBehaviorTree "/Game/Blueprints/AIEnemy/BT_EnemyAI.BT_EnemyAI"))

(event EventBeginPlay
  (bind _output_get (Variables|Default|SetGame%20State (.AsBP%20Game%20State%20Base (Utilities|Casting|CastToBP_GameStateBase (Game|GetGameState)))))
  (EventDispatchers|BindEventtoChangedGameState _output_get (EventDispatchers|CreateEvent :!event OnGameStateChange)))

(fn ConstructionScript)

(fn SelectPlayableCharacter
  (bind _outactors (Actor|GetAllActorsOfClasswithTag "/Script/Engine.Character" "Enemy"))
  (bind _asbp_player_character (Utilities|Casting|CastToBP_PlayerCharacter (Utilities|Array|Get(acopy) _outactors (Math|Random|RandomInteger (Utilities|Array|Length _outactors)))))
  (Default|SelectCharacter (Variables|Default|GetGame%20State) _asbp_player_character)
  (return _asbp_player_character))

(fn SelectTarget
  (bind _outactors (Actor|GetAllActorsOfClasswithTag "/Script/Engine.Character" "Player"))
  (bind _asbp_player_character (Utilities|Casting|CastToBP_PlayerCharacter (Utilities|Array|Get(acopy) _outactors (Math|Random|RandomInteger (Utilities|Array|Length _outactors)))))
  (return _asbp_player_character))

(fn SelectActiontoPlay
  (Default|SelectAction (Variables|Default|GetGame%20State) "NewEnumerator4")
  (return (Default|GetCurrentlySelectedAction (Variables|Default|GetGame%20State))))

(fn OnGameStateChange
  (AI|Components|Blackboard|SetValueasBool (Variables|Default|GetBlackboard) (Utilities|Name|MakeLiteralName "IsEnemyTurn") (Variables|/Game/Blueprints/BP_GameStateBase.BP_GameStateBase_C|GetIsEnemyTurn (Variables|Default|GetGame%20State))))

(fn EndTurn)

(fn PreviewAction
  (bind _game_state (Variables|Default|GetGame%20State))
  (Default|EnablePreviewforEnemy (Default|GetCurrentlySelectedAction _game_state) (.AsAIC%20Player%20Character (Utilities|Casting|CastToAIC_PlayerCharacter (AI|GetAIController (Variables|/Game/Blueprints/BP_GameStateBase.BP_GameStateBase_C|GetSelectedCharacter _game_state))))))

(fn PlayAction
  (bind _returnvalue (Utilities|Name|MakeLiteralName "TargetCharacter"))
  (bind _blackboard (Variables|Default|GetBlackboard))
  (bind _returnvalue_2 (AI|Components|Blackboard|GetValueasObject _blackboard _returnvalue))
  (bind _asbp_player_character (Utilities|Casting|CastToBP_PlayerCharacter (AI|Components|Blackboard|GetValueasObject (Variables|Default|GetBlackboard) (Utilities|Name|MakeLiteralName "PlayingCharacter"))))
  (bind _asbp_player_character_2 (Utilities|Casting|CastToBP_PlayerCharacter _returnvalue_2))
  (bind (_outhit _returnvalue_3) (Collision|LineTraceForObjects (Transformation|GetActorLocation _asbp_player_character) (Transformation|GetActorLocation _asbp_player_character_2) (Utilities|Array|MakeArray "ObjectTypeQuery7" "ObjectTypeQuery1") false (Utilities|Array|MakeArray _asbp_player_character) "None" true "(R=1.000000,G=0.000000,B=0.000000,A=1.000000)" "(R=0.000000,G=1.000000,B=0.000000,A=1.000000)" 0.5))
  (if (and _returnvalue_3 (== _returnvalue_2 (.HitActor (Collision|BreakHitResult _outhit))))
    (bind _outlaunchvelocity (Game|SuggestProjectileVelocityCustomArc (Transformation|GetActorLocation _asbp_player_character) (Transformation|GetActorLocation _asbp_player_character_2) 0.0 0.999))
    (bind _returnvalue_4 (Game|SpawnActorfromClass "/Game/Blueprints/BP_BasicProjectile.BP_BasicProjectile_C" (Math|Transform|MakeTransform (Transformation|GetActorLocation _asbp_player_character) "0, 0, 0" "1,1,1") "AlwaysSpawn" _asbp_player_character 0))
    (Components|Activation|Activate (Variables|/Game/Blueprints/BP_BasicProjectile.BP_BasicProjectile_C|GetProjectileMovement _returnvalue_4) true)
    (Game|Components|ProjectileMovement|SetVelocityinLocalSpace (Variables|/Game/Blueprints/BP_BasicProjectile.BP_BasicProjectile_C|GetProjectileMovement _returnvalue_4) _outlaunchvelocity)))