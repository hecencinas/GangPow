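; BPC_Interactable is an actor component that makes its owner clickable and highlightable with the mouse.
; On BeginPlay it binds to the owner's click event and to cursor-over events on the owner's first mesh component.
; Hovering turns on the mesh's custom depth rendering, and clicking toggles a selected state that keeps it on after the cursor leaves.
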(event Custom|OnClicked_Event
  (params (TouchedActor :type Actor%20Object%20Reference) (ButtonPressed :type Key%20Structure))
  (Variables|Default|SetIsSelected (not (Variables|Default|GetIsSelected))))

(event Custom|OnEndCursorOver_Event
  (params (TouchedComponent :type Primitive%20Component%20Object%20Reference))
  (if (not (Variables|Default|GetIsSelected))
    (Rendering|SetRenderCustomDepth (Variables|Default|GetOwnerMesh) false)))

(event Custom|OnBeginCursorOver_Event
  (params (TouchedComponent :type Primitive%20Component%20Object%20Reference))
  (Rendering|SetRenderCustomDepth (Variables|Default|GetOwnerMesh) true))

(event EventBeginPlay
  (bind _returnvalue (Components|GetOwner))
  (Variables|Default|SetPlayerController (Game|GetPlayerController 0))
  (EventDispatchers|AssignOnClicked _returnvalue (delegate Custom|OnClicked_Event))
  (bind _output_get (Variables|Default|SetOwnerMesh (Actor|GetComponentbyClass _returnvalue "/Script/Engine.MeshComponent")))
  (EventDispatchers|AssignOnBeginCursorOver _output_get (delegate Custom|OnBeginCursorOver_Event))
  (EventDispatchers|AssignOnEndCursorOver _output_get (delegate Custom|OnEndCursorOver_Event)))